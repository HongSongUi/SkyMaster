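; Game mode for the character death sequence, built around the damaged player character and its controller.
; On BeginPlay it caches the player character and controller, then sets IsPlayerDestroy on the game instance if all casts succeed.
; Every Tick, while the character's IsDestroy flag is set, it starts a strong world-space camera shake on the controller, re-triggering it each frame.
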(event EventBeginPlay
  (bind _asbp_damaged_char (Utilities|Casting|CastToBP_DamagedChar (Game|GetPlayerCharacter 0)))
  (Variables|Default|SetChar _asbp_damaged_char)
  (bind _asbp_damaged_char_con (Utilities|Casting|CastToBP_DamagedCharCon (Game|GetPlayerController 0)))
  (Variables|Default|SetController _asbp_damaged_char_con)
  (bind _asbp_game_inst (Utilities|Casting|CastToBP_GameInst (Game|GetGameInstance)))
  (Variables|/Game/BluePrint/InGame/BP_GameInst.BP_GameInst_C|SetIsPlayerDestroy _asbp_game_inst true))

(event EventTick
  (params (DeltaSeconds :type Float%20%28single-precision%29))
  (if (Variables|/Game/BluePrint/CharDie/BP_DamagedChar.BP_DamagedChar_C|GetIsDestroy (Variables|Default|GetChar))
    (Game|Feedback|ClientStartCameraShake (Variables|Default|GetController) "/Game/BluePrint/InGame/BP_CamGetForce.BP_CamGetForce_C" 1e+01 "World" "0, 0, 0")))

(fn ConstructionScript)