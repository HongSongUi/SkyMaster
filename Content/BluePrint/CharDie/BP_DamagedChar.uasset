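; BP_DamagedChar is a damaged character that plays a falling, spinning crash ending in a large explosion.
; BeginPlay switches movement to Flying, then Tick feeds forward-plus-downward input from control rotation, nudges the rotation once and spins the actor each frame.
; An accumulated timer triggers the explosion emitter and BigExplosion after four seconds, hides the mesh and stops further Tick logic without destroying the actor.
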(event EventBeginPlay
  (Pawn|Components|CharacterMovement|SetMovementMode (Variables|Character|GetCharacterMovement) "MOVE_Flying" 0))

(event Collision|EventActorBeginOverlap
  (params (OtherActor :type Actor%20Object%20Reference)))

(event EventTick
  (params (DeltaSeconds :type Float%20%28single-precision%29))
  (bind _returnvalue (Pawn|GetControlRotation :!class /Script/Engine.Pawn))
  (if (not (Variables|Default|GetIsDestroy))
    (Utilities|FlowControl|Sequence
      (:then_0
        (Variables|Default|SetDelta%20Seconds DeltaSeconds)
        (Variables|Default|SetSecondPerFrame (+ (Variables|Default|GetDelta%20Seconds) (Variables|Default|GetSecondPerFrame))))
      (:then_1
        (Pawn|Input|AddMovementInput (+ (Math|Vector|GetForwardVector (Math|Rotator|MakeRotator (.roll _returnvalue) 0.0 (.yaw _returnvalue))) (* (Math|Vector|GetUpVector (Math|Rotator|MakeRotator (.roll _returnvalue) 0.0 (.yaw _returnvalue))) -1.0)) 1.0 false))
      (:then_2
        (if (not (Variables|Default|GetSetRotation))
          (Transformation|SetActorRotation (Math|Interpolation|RInterpTo (Pawn|GetControlRotation :!class /Script/Engine.Pawn) "-40.000000, 0,0.000000" (Variables|Default|GetDelta%20Seconds) 0.0))
          (Variables|Default|SetSetRotation true)))
      (:then_3
        (Transformation|AddActorLocalRotation "0.000000,0.000000,5.000000" false false))
      (:then_4
        (if (>= (Variables|Default|GetSecondPerFrame) 4.0)
          (Effects|SpawnEmitteratLocation "/Game/ExplosionB/Particles/Explosion/P_Explosion_Big_B.P_Explosion_Big_B" (Transformation|GetActorLocation) "0, 0, 0" "20.000000,20.000000,20.000000")
          (Rendering|SetVisibility (Variables|Character|GetMesh) false true)
          (Audio|Components|Audio|Play (Variables|Default|GetBigExplosion) 0.0)
          (Variables|Default|SetIsDestroy true))))))

(fn ConstructionScript)