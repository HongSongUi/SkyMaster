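; BP_Ending is the ending-sequence Character for an aircraft-like craft with canopy, nozzle and wheels, controlled through BP_EndingCont.
; BeginPlay caches ABP_Char and the controller, enables Flying movement and raises emission on the mesh's dynamic material.
; Tick drives it forward and downward until IsLanding, applying a single RInterpTo rotation step on the first pass.
; Canopy, nozzle and wheel helpers animate AnimInstance values but are not called within this Blueprint.
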(event EventBeginPlay
  (bind _asabp_char (Utilities|Casting|CastToABP_Char (Components|SkeletalMesh|GetAnimInstance (Variables|Character|GetMesh))))
  (bind _output_get (Variables|Default|SetAnimInstance _asabp_char))
  (Variables|/Game/Animation/ABP_Char.ABP_Char_C|SetCanopy _output_get 0.0)
  (bind _asbp_ending_cont (Utilities|Casting|CastToBP_EndingCont (Game|GetPlayerController 0)))
  (Variables|Default|SetPlayerCon _asbp_ending_cont)
  (Pawn|Components|CharacterMovement|SetMovementMode (Variables|Character|GetCharacterMovement) "MOVE_Flying" 0)
  (CallFunction|SetLight))

(event Collision|EventActorBeginOverlap
  (params (OtherActor :type Actor%20Object%20Reference)))

(event EventTick
  (params (DeltaSeconds :type Float%20%28single-precision%29))
  (bind _returnvalue (Pawn|GetControlRotation :!class /Script/Engine.Pawn))
  (Utilities|FlowControl|Sequence
    (:then_0
      (Variables|Default|SetDelta%20Seconds DeltaSeconds)
      (Variables|Default|SetSecondPerFrame (+ (Variables|Default|GetDelta%20Seconds) (Variables|Default|GetSecondPerFrame))))
    (:then_1
      (if (not (Variables|Default|GetIsLanding))
        (Pawn|Input|AddMovementInput (+ (Math|Vector|GetForwardVector (Math|Rotator|MakeRotator (.roll _returnvalue) 0.0 (.yaw _returnvalue))) (* (Math|Vector|GetUpVector (Math|Rotator|MakeRotator (.roll _returnvalue) 0.0 (.yaw _returnvalue))) -1.0)) 1.0 false)))
    (:then_2
      (if (not (Variables|Default|GetSetRotation))
        (Transformation|SetActorRotation (Math|Interpolation|RInterpTo (Pawn|GetControlRotation :!class /Script/Engine.Pawn) "-40.000000, 0,0.000000" (Variables|Default|GetDelta%20Seconds) 0.0))
        (Variables|Default|SetSetRotation true)))
    (:then_3
      (if (Variables|Default|GetIsBreak)
        _))))

(fn ConstructionScript
  (|CallParentFunction)
  (bind _returnvalue (Rendering|Material|CreateDynamicMaterialInstance (Variables|Character|GetMesh) 0 0 "None" :!class /Script/Engine.PrimitiveComponent))
  (Variables|Default|SetLight _returnvalue))

(fn CloseCanopy
  (bind _animinstance (Variables|Default|GetAnimInstance))
  (bind _output_get (Variables|/Game/Animation/ABP_Char.ABP_Char_C|SetCanopy _animinstance (Math|Float|Lerp (Variables|/Game/Animation/ABP_Char.ABP_Char_C|GetCanopy _animinstance) 0.0 (Variables|Default|GetDelta%20Seconds)))))

(fn SetLight
  (Rendering|Material|SetScalarParameterValue (Variables|Default|GetLight) "Emission" 1e+02 :!class /Script/Engine.MaterialInstanceDynamic))

(fn NozzleSet
  (bind _animinstance (Variables|Default|GetAnimInstance))
  (Variables|/Game/Animation/ABP_Char.ABP_Char_C|SetFireNozzle _animinstance (Math|Float|SelectFloat 1.0 (+ 0.0025 (Variables|/Game/Animation/ABP_Char.ABP_Char_C|GetFireNozzle _animinstance)) (>= (+ 0.0025 (Variables|/Game/Animation/ABP_Char.ABP_Char_C|GetFireNozzle _animinstance)) 1.0)))
  (if (>= (Math|Float|SelectFloat 1.0 (+ 0.0025 (Variables|/Game/Animation/ABP_Char.ABP_Char_C|GetFireNozzle _animinstance)) (>= (+ 0.0025 (Variables|/Game/Animation/ABP_Char.ABP_Char_C|GetFireNozzle _animinstance)) 1.0)) 1.0)
    _))

(fn WheelSet
  (bind _animinstance (Variables|Default|GetAnimInstance))
  (bind _delta_seconds (Variables|Default|GetDelta%20Seconds))
  (Variables|/Game/Animation/ABP_Char.ABP_Char_C|SetFrontWheel _animinstance (Math|Float|Lerp (Variables|/Game/Animation/ABP_Char.ABP_Char_C|GetFrontWheel _animinstance) 0.0 _delta_seconds))
  (Variables|/Game/Animation/ABP_Char.ABP_Char_C|SetRearWheel _animinstance (Math|Float|Lerp (Variables|/Game/Animation/ABP_Char.ABP_Char_C|GetRearWheel _animinstance) 0.0 _delta_seconds)))