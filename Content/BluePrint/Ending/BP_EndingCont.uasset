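; BP_EndingCont is a controller for the game's ending that automatically steers the player character once it has landed.
; BeginPlay caches the character; while IsLanding is set, Tick smoothly levels its pitch and roll with RInterpTo, keeping its current yaw.
; Unless IsBreak is set, it also pushes the character forward along the flattened control-rotation direction.
; Neither flag is set within this Blueprint.
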(event EventBeginPlay
  (Variables|Default|Setchar (Game|GetPlayerCharacter 0)))

(event EventTick
  (params (DeltaSeconds :type Float%20%28single-precision%29))
  (bind _returnvalue (Pawn|GetControlRotation :!class /Script/Engine.Controller))
  (bind _char (Variables|Default|Getchar))
  (if (Variables|Default|GetIsLanding)
    (Transformation|SetActorRotation _char (Math|Interpolation|RInterpTo (Transformation|GetActorRotation _char) (Math|Rotator|MakeRotator 0.0 0.0 (.yaw (Transformation|GetActorRotation _char))) DeltaSeconds 2.0))
    (if (not (Variables|Default|GetIsBreak))
      (Pawn|Input|AddMovementInput (Variables|Default|Getchar) (Math|Vector|GetForwardVector (Math|Rotator|MakeRotator (.roll _returnvalue) 0.0 (.yaw _returnvalue))) 1.0 false))))

(fn ConstructionScript)