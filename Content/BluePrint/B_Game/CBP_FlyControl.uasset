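; Flight controller that drives the player's BP_Fly character through an automatic forward run and takeoff, with engine effects.
; Each Tick pushes it forward along control yaw while its IsPreEnd flag is set, and toggles two thruster emitters on mesh sockets based on speed.
; InTrigger, never set here, switches movement to Flying with forward-plus-up input.
; This latches Flying, which eases actor rotation toward a fixed tilt.
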(event EventBeginPlay
  (bind _returnvalue (Game|GetPlayerCharacter 0))
  ;[1 1 1] BeginPlay
  (bind _output_get (Variables|Default|SetFlyPlayer _returnvalue))
  (Variables|Default|SetCharMovement (Variables|/Script/Engine.Character|GetCharacterMovement _output_get))
  (bind _asbp_fly (Utilities|Casting|CastToBP_Fly _returnvalue))
  (Variables|Default|SetChar _asbp_fly))

(event EventTick
  (params (DeltaSeconds :type Float%20%28single-precision%29))
  (bind _flyplayer (Variables|Default|GetFlyPlayer))
  (bind _flyplayer_2 (Variables|Default|GetFlyPlayer))
  (bind _returnvalue (Pawn|GetControlRotation _flyplayer :!class /Script/Engine.Pawn))
  (bind _mesh (Variables|/Script/Engine.Character|GetMesh _flyplayer_2))
  (Variables|Default|SetDelta%20Seconds DeltaSeconds)
  (Utilities|FlowControl|Sequence
    (:then_0
      ;[1 1 1] Forward/Back
      (if (Variables|/Game/BluePrint/B_Game/BP_Fly.BP_Fly_C|GetIsPreEnd (Variables|Default|GetChar))
        (Pawn|Input|AddMovementInput _flyplayer (Math|Vector|GetForwardVector (Math|Rotator|MakeRotator 0.0 0.0 (.yaw (Pawn|GetControlRotation _flyplayer :!class /Script/Engine.Pawn)))) 1.0 false)))
    (:then_1
      ;[1 1 1] SetVelocity
      (Variables|Default|SetVelocity (Math|Vector|VectorLength (Transformation|GetVelocity _flyplayer))))
    (:then_2
      ;[1 1 1] Effect
      (if (> (Variables|Default|GetVelocity) 1.0)
        (Utilities|IsValid (Variables|Default|GetLeftFire)
          (:Is%20Not%20Valid
            (Utilities|IsValid (Variables|Default|GetRightFire)
              (:Is%20Not%20Valid
                (Utilities|FlowControl|Sequence
                  (:then_0
                    (bind _returnvalue_2 (Effects|SpawnEmitterAttached "/Game/InGameVigilante/Vehicles/West_Fighter_F18C/FX/FX_Engine_01_F18C.FX_Engine_01_F18C" _mesh "lf_thruster_jntSocket"))
                    (Variables|Default|SetLeftFire _returnvalue_2))
                  (:then_1
                    (bind _returnvalue_3 (Effects|SpawnEmitterAttached "/Game/InGameVigilante/Vehicles/West_Fighter_F18C/FX/FX_Engine_01_F18C.FX_Engine_01_F18C" _mesh "rt_thruster_jntSocket"))
                    (Variables|Default|SetRightFire _returnvalue_3)))))))
        (else
          (Utilities|IsValid (Variables|Default|GetLeftFire)
            (:Is%20Valid
              (Utilities|IsValid (Variables|Default|GetRightFire)
                (:Is%20Valid
                  (Components|DestroyComponent (Variables|Default|GetRightFire))
                  (Components|DestroyComponent (Variables|Default|GetLeftFire)))))))))
    (:then_3
      ;[1 1 1] Flying
      (if (Variables|Default|GetInTrigger)
        (Pawn|Components|CharacterMovement|SetMovementMode (Variables|Default|GetCharMovement) "MOVE_Flying" 0)
        (Pawn|Input|AddMovementInput _flyplayer (+ (Math|Vector|GetForwardVector (Math|Rotator|MakeRotator (.roll _returnvalue) 0.0 (.yaw _returnvalue))) (Math|Vector|GetUpVector (Math|Rotator|MakeRotator (.roll _returnvalue) 0.0 (.yaw _returnvalue)))) 1.0 false)
        (Variables|Default|SetFlying true)))
    (:then_4
      ;[1 1 1] Rotation
      (if (Variables|Default|GetFlying)
        (Transformation|SetActorRotation _flyplayer (Math|Interpolation|RInterpTo (Transformation|GetActorRotation _flyplayer) "25.000000, 0, 0" (Variables|Default|GetDelta%20Seconds) 2.0))))))

(fn ConstructionScript)