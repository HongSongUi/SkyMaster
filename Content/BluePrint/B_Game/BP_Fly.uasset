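; BP_Fly is a flyable aircraft that plays a boarding and engine start-up sequence from an intro widget with flashing text.
; Space sets Riding, switching to the interior camera while Tick lerps the anim instance's canopy closed.
; Closing ramps a dynamic material's emission, then restores the exterior camera, opens nozzles, swaps engine effects and sets StartMove.
; The controller's Flying flag drives the wheel animation.
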(event EventBeginPlay
  (bind _asabp_char (Utilities|Casting|CastToABP_Char (Components|SkeletalMesh|GetAnimInstance (Variables|Character|GetMesh))))
  (bind _output_get (Variables|Default|SetAnimInstance _asabp_char))
  (Variables|/Game/Animation/ABP_Char.ABP_Char_C|SetCanopy _output_get 9e+01)
  (bind _ascbp_fly_control (Utilities|Casting|CastToCBP_FlyControl (Pawn|GetController)))
  (Variables|Default|SetControl _ascbp_fly_control)
  (bind _returnvalue (UserInterface|CreateWidget "/Game/UI/BP_Intro.BP_Intro_C"))
  (bind _output_get_2 (Variables|Default|SetWidget _returnvalue))
  (UserInterface|Viewport|AddtoViewport _output_get_2 0))

(event Collision|EventActorBeginOverlap
  (params (OtherActor :type Actor%20Object%20Reference)))

(event EventTick
  (params (DeltaSeconds :type Float%20%28single-precision%29))
  (bind _engine (Variables|Default|GetEngine))
  (bind _widget (Variables|Default|GetWidget))
  (Utilities|FlowControl|Sequence
    (:then_0
      (CallFunction|CloseCanopy)
      (if (Variables|Default|GetIsClose)
        (CallFunction|SetLight)
        (if (Variables|Default|GetLightEnd)
          (CallFunction|NozzleSet))))
    (:then_1
      (if (Variables|/Game/BluePrint/B_Game/CBP_FlyControl.CBP_FlyControl_C|GetFlying (Variables|Default|GetControl))
        (CallFunction|WheelSet)))
    (:then_2
      (if (Variables|Default|GetRiding)
        (Widget|SetVisibility (Variables|/Game/UI/BP_Intro.BP_Intro_C|GetSpace _widget) "Hidden")
        (elif (not (Class|UserWidget|IsPlayingAnimation _widget))
          (Class|UserWidget|PlayAnimationForward _widget (Variables|/Game/UI/BP_Intro.BP_Intro_C|GetFlashText _widget) 1.0 false))))
    (:then_3
      (if (Variables|Default|GetLightEnd)
        (if (Variables|Default|GetFireSound)
          (Variables|Default|SetStartMove true)
          (Utilities|FlowControl|Delay 1.0)
          (Components|Activation|SetActive _engine false false)
          (else
            (Components|Activation|SetActive _engine true false)
            (Variables|Default|SetFireSound true)
            (Components|Activation|SetActive (Variables|Default|GetEngineBefore) false false)))
        (else
          (Components|Activation|SetActive (Variables|Default|GetEngineBefore) true false))))))

(event Input|KeyboardEvents|SpaceBar
  (params (Key :type Key%20Structure :default "None"))
  (:Pressed
    (Audio|PlaySound2D "/Game/Sound/Space_bar.Space_bar" 1.0 1.0 0.0 0 0)
    (Utilities|FlowControl|Delay 0.2)
    (Variables|Default|SetRiding true)))

(fn ConstructionScript
  (|CallParentFunction)
  (bind _returnvalue (Rendering|Material|CreateDynamicMaterialInstance (Variables|Character|GetMesh) 0 0 "None" :!class /Script/Engine.PrimitiveComponent))
  (Variables|Default|SetLight _returnvalue))

(fn CloseCanopy
  (bind _animinstance (Variables|Default|GetAnimInstance))
  (if (Variables|Default|GetRiding)
    (Components|Activation|Activate (Variables|Default|GetInCamera) false)
    (Components|Activation|Deactivate (Variables|Camera|GetOutCamera))
    (bind _output_get (Variables|/Game/Animation/ABP_Char.ABP_Char_C|SetCanopy _animinstance (Math|Float|Lerp (Variables|/Game/Animation/ABP_Char.ABP_Char_C|GetCanopy _animinstance) 0.0 (Variables|Default|GetDelta%20Seconds))))
    (Variables|Default|SetIsClose (< _output_get 0.5))))

(fn SetLight
  (if (<= (Variables|Default|GetLightValue) 1e+02)
    (bind _output_get (Variables|Default|SetLightValue (* (Variables|Default|GetSecondPerFrame) 7.0))))
  (Rendering|Material|SetScalarParameterValue (Variables|Default|GetLight) "Emission" (Math|Float|SelectFloat _output_get (Variables|Default|GetLightValue) (<= (Variables|Default|GetLightValue) 1e+02)) :!class /Script/Engine.MaterialInstanceDynamic)
  (if (>= (Variables|Default|GetLightValue) 8e+01)
    (Variables|Default|SetLightEnd true)
    (Components|Activation|Activate (Variables|Camera|GetOutCamera) false)
    (Components|Activation|Deactivate (Variables|Default|GetInCamera))))

(fn NozzleSet
  (bind _animinstance (Variables|Default|GetAnimInstance))
  (Variables|/Game/Animation/ABP_Char.ABP_Char_C|SetFireNozzle _animinstance (Math|Float|SelectFloat 1.0 (+ 0.0025 (Variables|/Game/Animation/ABP_Char.ABP_Char_C|GetFireNozzle _animinstance)) (>= (+ 0.0025 (Variables|/Game/Animation/ABP_Char.ABP_Char_C|GetFireNozzle _animinstance)) 1.0)))
  (if (>= (Math|Float|SelectFloat 1.0 (+ 0.0025 (Variables|/Game/Animation/ABP_Char.ABP_Char_C|GetFireNozzle _animinstance)) (>= (+ 0.0025 (Variables|/Game/Animation/ABP_Char.ABP_Char_C|GetFireNozzle _animinstance)) 1.0)) 1.0)
    (Variables|Default|SetIsPreEnd true)))

(fn WheelSet
  (bind _animinstance (Variables|Default|GetAnimInstance))
  (bind _delta_seconds (Variables|Default|GetDelta%20Seconds))
  (Variables|/Game/Animation/ABP_Char.ABP_Char_C|SetFrontWheel _animinstance (Math|Float|Lerp (Variables|/Game/Animation/ABP_Char.ABP_Char_C|GetFrontWheel _animinstance) 1.0 _delta_seconds))
  (Variables|/Game/Animation/ABP_Char.ABP_Char_C|SetRearWheel _animinstance (Math|Float|Lerp (Variables|/Game/Animation/ABP_Char.ABP_Char_C|GetRearWheel _animinstance) 1.0 _delta_seconds)))