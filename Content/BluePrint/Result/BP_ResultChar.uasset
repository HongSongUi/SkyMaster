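; BP_ResultChar is a result character actor that reflects the player's state as stored in the game instance.
; On BeginPlay it casts to BP_GameInst and, if the player is destroyed, hides the mesh and shows the Destroy component and particle system.
; Otherwise it moves and rotates itself to the saved player position and rotation.
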(event EventBeginPlay
  (bind _asbp_game_inst (Utilities|Casting|CastToBP_GameInst (Game|GetGameInstance)))
  (Variables|Default|SetGameInst _asbp_game_inst)
  (if (Variables|/Game/BluePrint/InGame/BP_GameInst.BP_GameInst_C|GetIsPlayerDestroy (Variables|Default|GetGameInst))
    (Rendering|SetVisibility (Variables|Default|GetDestroy) true false)
    (Rendering|SetVisibility (Variables|Character|GetMesh) false false)
    (Rendering|SetVisibility (Variables|Default|GetParticleSystem) true false)
    (else
      (Transformation|SetActorLocation (Variables|/Game/BluePrint/InGame/BP_GameInst.BP_GameInst_C|GetPlayerPos (Variables|Default|GetGameInst)) false false)
      (Transformation|SetActorRotation (Variables|/Game/BluePrint/InGame/BP_GameInst.BP_GameInst_C|GetPlayerRotation (Variables|Default|GetGameInst))))))

(event Collision|EventActorBeginOverlap
  (params (OtherActor :type Actor%20Object%20Reference)))

(event EventTick
  (params (DeltaSeconds :type Float%20%28single-precision%29)))

(fn ConstructionScript)