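; Game mode for the result screen that shows mission outcome, score, damage taken and a letter rank.
; On BeginPlay it creates the BP_Result widget and fills it from the values stored in BP_GameInst.
; A destroyed player gets red MISSION FAILED, zeroed numbers and rank F with no sound.
; Otherwise score minus a damage penalty sets rank D to SS, with a lose or win sound.
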(event EventBeginPlay
  (Variables|/Script/Engine.PlayerController|SetbShowMouseCursor (Game|GetPlayerController 0) true)
  (bind _asbp_result_char (Utilities|Casting|CastToBP_ResultChar (Game|GetPlayerCharacter 0)))
  (Variables|Default|SetChar _asbp_result_char)
  (bind _returnvalue (UserInterface|CreateWidget "/Game/UI/BP_Result.BP_Result_C"))
  (bind _output_get (Variables|Default|SetResult _returnvalue))
  (UserInterface|Viewport|AddtoViewport _output_get 0)
  (bind _asbp_game_inst (Utilities|Casting|CastToBP_GameInst (Game|GetGameInstance)))
  (Variables|Default|SetGameInst _asbp_game_inst)
  (CallFunction|SetMission)
  (CallFunction|SetResultText)
  (if (Variables|/Game/BluePrint/InGame/BP_GameInst.BP_GameInst_C|GetIsPlayerDestroy (Variables|Default|GetGameInst))
    (Rendering|Components|TextRender|SetText (Variables|/Game/UI/BP_Result.BP_Result_C|GetRANK (Variables|Default|GetResult)) "F")
    (Appearance|SetColorandOpacity (Variables|/Game/UI/BP_Result.BP_Result_C|GetRANK (Variables|Default|GetResult)) (Utilities|Struct|MakeSlateColor "(R=1.000000,G=0.000000,B=0.000000,A=1.000000)" "UseColor_Specified") :!class /Script/UMG.TextBlock)
    (else
      (bind _output_get_2 (Variables|Default|SetTotalScore (+ (* (Variables|/Game/BluePrint/InGame/BP_GameInst.BP_GameInst_C|GetDamaged (Variables|Default|GetGameInst)) -10) (+ (Variables|/Game/BluePrint/InGame/BP_GameInst.BP_GameInst_C|GetScore (Variables|Default|GetGameInst)) 0))))
      (if (<= _output_get_2 200)
        (Rendering|Components|TextRender|SetText (Variables|/Game/UI/BP_Result.BP_Result_C|GetRANK (Variables|Default|GetResult)) "D")
        (Audio|Components|Audio|Play (Variables|Default|GetLoseSound) 0.0 :!label _label)
        (elif (<= (Variables|Default|GetTotalScore) 300)
          (Rendering|Components|TextRender|SetText (Variables|/Game/UI/BP_Result.BP_Result_C|GetRANK (Variables|Default|GetResult)) "C")
          (goto _label)
          (elif (<= (Variables|Default|GetTotalScore) 400)
            (Rendering|Components|TextRender|SetText (Variables|/Game/UI/BP_Result.BP_Result_C|GetRANK (Variables|Default|GetResult)) "B")
            (Audio|Components|Audio|Play (Variables|Default|GetWinSound) 0.0 :!label _label_2)
            (elif (<= (Variables|Default|GetTotalScore) 500)
              (Rendering|Components|TextRender|SetText (Variables|/Game/UI/BP_Result.BP_Result_C|GetRANK (Variables|Default|GetResult)) "A")
              (goto _label_2)
              (elif (<= (Variables|Default|GetTotalScore) 600)
                (Rendering|Components|TextRender|SetText (Variables|/Game/UI/BP_Result.BP_Result_C|GetRANK (Variables|Default|GetResult)) "S")
                (goto _label_2)
                (elif (> (Variables|Default|GetTotalScore) 600)
                  (Rendering|Components|TextRender|SetText (Variables|/Game/UI/BP_Result.BP_Result_C|GetRANK (Variables|Default|GetResult)) "SS")
                  (goto _label_2))))))))))

(event EventTick
  (params (DeltaSeconds :type Float%20%28single-precision%29)))

(fn ConstructionScript)

(fn SetMission
  (bind _result (Variables|Default|GetResult))
  (bind _result_2 (Variables|Default|GetResult))
  (bind _result_3 (Variables|Default|GetResult))
  (bind _result_4 (Variables|Default|GetResult))
  (bind _result_5 (Variables|Default|GetResult))
  (if (Variables|/Game/BluePrint/InGame/BP_GameInst.BP_GameInst_C|GetIsPlayerDestroy (Variables|Default|GetGameInst))
    (Appearance|SetColorandOpacity (Variables|/Game/UI/BP_Result.BP_Result_C|GetMission_1 _result_3) (Utilities|Struct|MakeSlateColor "(R=1.000000,G=0.000000,B=0.000000,A=1.000000)" "UseColor_Specified") :!class /Script/UMG.TextBlock)
    (Appearance|SetColorandOpacity (Variables|/Game/UI/BP_Result.BP_Result_C|GetMission_0 _result_3) (Utilities|Struct|MakeSlateColor "(R=1.000000,G=0.000000,B=0.000000,A=1.000000)" "UseColor_Specified") :!class /Script/UMG.TextBlock)
    (Rendering|Components|TextRender|SetText (Variables|/Game/UI/BP_Result.BP_Result_C|GetMission_0 _result_5) "MISSION")
    (Rendering|Components|TextRender|SetText (Variables|/Game/UI/BP_Result.BP_Result_C|GetMission_1 _result_5) "FAILED")
    (else
      (Appearance|SetColorandOpacity (Variables|/Game/UI/BP_Result.BP_Result_C|GetMission_0 _result) (Utilities|Struct|MakeSlateColor "(R=0.000000,G=1.000000,B=0.000000,A=1.000000)" "UseColor_Specified") :!class /Script/UMG.TextBlock)
      (Appearance|SetColorandOpacity (Variables|/Game/UI/BP_Result.BP_Result_C|GetMission_1 _result) (Utilities|Struct|MakeSlateColor "(R=0.000000,G=1.000000,B=0.000000,A=1.000000)" "UseColor_Specified") :!class /Script/UMG.TextBlock)
      (Rendering|Components|TextRender|SetText (Variables|/Game/UI/BP_Result.BP_Result_C|GetMission_0 _result_2) "MISSON")
      (Rendering|Components|TextRender|SetText (Variables|/Game/UI/BP_Result.BP_Result_C|GetMission_1 _result_2) "SUCCESS")))
  (Widget|SetVisibility (Variables|/Game/UI/BP_Result.BP_Result_C|GetMission_1 _result_4) "Visible")
  (Widget|SetVisibility (Variables|/Game/UI/BP_Result.BP_Result_C|GetMission_0 _result_4) "Visible"))

(fn SetResultText
  (bind _result (Variables|Default|GetResult))
  (bind _gameinst (Variables|Default|GetGameInst))
  (bind _numscore (Variables|/Game/UI/BP_Result.BP_Result_C|GetNumScore _result))
  (bind _numdamaged (Variables|/Game/UI/BP_Result.BP_Result_C|GetNumDamaged _result))
  (if (Variables|/Game/BluePrint/InGame/BP_GameInst.BP_GameInst_C|GetIsPlayerDestroy (Variables|Default|GetGameInst))
    (Rendering|Components|TextRender|SetText _numscore "0")
    (Rendering|Components|TextRender|SetText _numdamaged "0")
    (else
      (Rendering|Components|TextRender|SetText _numscore (Utilities|Text|ToText(Integer) (Variables|/Game/BluePrint/InGame/BP_GameInst.BP_GameInst_C|GetScore _gameinst)))
      (Rendering|Components|TextRender|SetText _numdamaged (Utilities|Text|ToText(Integer) (Variables|/Game/BluePrint/InGame/BP_GameInst.BP_GameInst_C|GetDamaged _gameinst)))
      (return))))