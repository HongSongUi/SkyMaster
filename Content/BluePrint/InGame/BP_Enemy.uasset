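; Enemy fighter jet for an in-game flight shooter, with flying movement and engine emitters attached to both turbines.
; Tick moves it along negative X unless it spawned behind the player; passing the player flags a miss, destroys it and deducts score.
; It spawns a single projectile from its socket once the player is within range.
; While IsAiming is set, an aim widget tracks its projected screen position.
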(event EventBeginPlay
  (bind _mesh (Variables|Character|GetMesh))
  (Utilities|FlowControl|Sequence
    (:then_0
      (Pawn|Components|CharacterMovement|SetMovementMode (Variables|Character|GetCharacterMovement) "MOVE_Flying" 0)
      (bind _asbp_in_game_char (Utilities|Casting|CastToBP_InGameChar (Game|GetPlayerCharacter 0)))
      (Variables|Default|SetPlayer _asbp_in_game_char)
      (bind _asgm_in_game (Utilities|Casting|CastToGM_InGame (Game|GetGameMode)))
      (Variables|Default|SetGameMode _asgm_in_game)
      (bind _returnvalue (UserInterface|CreateWidget "/Game/UI/BP_AimAttack.BP_AimAttack_C"))
      (bind _output_get (Variables|Default|SetAim _returnvalue))
      (UserInterface|Viewport|AddtoViewport _output_get 0)
      (Widget|SetVisibility (Variables|Default|GetAim) "Hidden")
      (bind _asabp_enemy (Utilities|Casting|CastToABP_Enemy (Components|SkeletalMesh|GetAnimInstance (Variables|Character|GetMesh))))
      (Variables|Default|SetAnimInstance _asabp_enemy)
      (Components|SkinnedMesh|SetPhysicsAsset (Variables|Character|GetMesh) "/Game/EnemyFly/Vehicles/East_Fighter_Su30/PHYS_East_Fighter_Su30.PHYS_East_Fighter_Su30" false)
      (Utilities|IsValid (Variables|Default|GetLeftFire)
        (:Is%20Not%20Valid
          (Utilities|IsValid (Variables|Default|GetRightFire)
            (:Is%20Not%20Valid
              (Utilities|FlowControl|Sequence
                (:then_0
                  (bind _returnvalue_2 (Effects|SpawnEmitterAttached "/Game/InGameVigilante/Vehicles/West_Fighter_F18C/FX/FX_Engine_01_F18C.FX_Engine_01_F18C" _mesh "lf_turbine_jnt" "0, 0, 0" "0,-180.000000, 0"))
                  (Variables|Default|SetLeftFire _returnvalue_2))
                (:then_1
                  (bind _returnvalue_3 (Effects|SpawnEmitterAttached "/Game/InGameVigilante/Vehicles/West_Fighter_F18C/FX/FX_Engine_01_F18C.FX_Engine_01_F18C" _mesh "rt_turbine_jnt" "0, 0, 0" "0,-180.000000, 0"))
                  (Variables|Default|SetRightFire _returnvalue_3))))))))
    (:then_1
      (Variables|Default|SetIsPlayerBack (< (.x (- (Transformation|GetActorLocation) (Transformation|GetActorLocation (Variables|Default|GetPlayer)))) 0.0)))))

(event EventTick
  (params (DeltaSeconds :type Float%20%28single-precision%29))
  (bind _gamemode (Variables|Default|GetGameMode))
  (Utilities|FlowControl|Sequence
    (:then_0
      (Variables|Default|SetDelta%20Seconds DeltaSeconds))
    (:then_1
      (if (Variables|Default|GetIsAiming)
        (Class|UserWidget|SetPositioninViewport (Variables|Default|GetAim) (.ScreenLocation (Class|PlayerController|ProjectWorldLocationtoScreen (Game|GetPlayerController 0) (Transformation|GetActorLocation) true)) true)
        (Widget|SetVisibility (Variables|Default|GetAim) "Visible")
        (Class|UserWidget|SetAlignmentinViewport (Variables|Default|GetAim) "(X=0.500000,Y=0.500000)")
        (else
          (Widget|SetVisibility (Variables|Default|GetAim) "Hidden"))))
    (:then_2
      (if (not (Variables|Default|GetIsPlayerBack))
        (Transformation|SetActorLocation (- (Transformation|GetActorLocation) (Math|Vector|MakeVector (.x (* (Variables|Default|GetDelta%20Seconds) (Variables|/Script/Engine.CharacterMovementComponent|GetMaxFlySpeed (Variables|Character|GetCharacterMovement)))) 0.0 0.0)) false false)
        (if (< (.x (- (Transformation|GetActorLocation) (Transformation|GetActorLocation (Variables|Default|GetPlayer)))) 0.0)
          (Variables|/Game/BluePrint/InGame/BP_InGameChar.BP_InGameChar_C|SetIsMiss (Variables|Default|GetPlayer) true)
          (Actor|DestroyActor)
          (Variables|/Game/BluePrint/InGame/GM_InGame.GM_InGame_C|SetScore _gamemode (- (Variables|/Game/BluePrint/InGame/GM_InGame.GM_InGame_C|GetScore _gamemode) 100)))))
    (:then_3
      (if (<= (Math|Vector|Distance(Vector) (Transformation|GetActorLocation) (Transformation|GetActorLocation (Variables|Default|GetPlayer))) 1e+05)
        (if (not (Variables|Default|GetSpawnProj))
          (Game|SpawnActorfromClass "/Game/BluePrint/InGame/SpawnEnemyProj.SpawnEnemyProj_C" (Math|Transform|MakeTransform (Transformation|GetSocketLocation (Variables|Character|GetMesh) "ProjSocket") "0, 0, 0" "1.000000,1.000000,1.000000") "AlwaysSpawn" 0 0)
          (Variables|Default|SetSpawnProj true))))))

(fn ConstructionScript)