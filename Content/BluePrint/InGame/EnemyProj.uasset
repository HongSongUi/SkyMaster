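; Enemy homing missile that chases the player character and resolves damage and score on impact.
; BeginPlay aims ProjectileMovement homing at the player with very high acceleration.
; Tick turns on the GameMode text flag at close range and drives the player's back-mirror flag when the missile trails in X within sight range.
; Player hits either damage, apply force and cost score, or award score when CanHit is false, then destroy the missile.
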(event EventBeginPlay
  (bind _projectilemovement (Variables|Default|GetProjectileMovement))
  (bind _asbp_game_inst (Utilities|Casting|CastToBP_GameInst (Game|GetGameInstance)))
  (Variables|Default|SetAs%20BP%20Game%20Inst _asbp_game_inst)
  (bind _asbp_in_game_char (Utilities|Casting|CastToBP_InGameChar (Game|GetPlayerCharacter 0)))
  (Variables|Default|SetTarget _asbp_in_game_char)
  (Components|SkinnedMesh|SetPhysicsAsset (Variables|Default|GetSkeletalMesh) "/Game/InGameVigilante/Projectiles/West_Missile_AGM114/PHYS_West_Missile_AGM114.PHYS_West_Missile_AGM114" false)
  (Variables|/Script/Engine.ProjectileMovementComponent|SetHomingTargetComponent _projectilemovement (Variables|/Script/Engine.Actor|GetRootComponent (Variables|Default|GetTarget)))
  (Variables|/Script/Engine.ProjectileMovementComponent|SetbIsHomingProjectile _projectilemovement true)
  (Variables|/Script/Engine.ProjectileMovementComponent|SetHomingAccelerationMagnitude _projectilemovement 4e+05)
  (bind _asbp_game_inst_2 (Utilities|Casting|CastToBP_GameInst (Game|GetGameInstance)))
  (Variables|Default|SetGameInst _asbp_game_inst_2)
  (bind _asgm_in_game (Utilities|Casting|CastToGM_InGame (Game|GetGameMode)))
  (Variables|Default|SetGameMode _asgm_in_game))

(event EventTick
  (params (DeltaSeconds :type Float%20%28single-precision%29))
  (bind _returnvalue (Transformation|GetActorLocation))
  (bind _target (Variables|Default|GetTarget))
  (bind _target_2 (Variables|Default|GetTarget))
  (bind _returnvalue_2 (Transformation|GetActorLocation _target_2))
  (Utilities|FlowControl|Sequence
    (:then_0
      (if (<= (Math|Vector|Distance(Vector) (Transformation|GetActorLocation) (Transformation|GetActorLocation (Variables|Default|GetTarget))) 1.45e+04)
        (Variables|/Game/BluePrint/InGame/GM_InGame.GM_InGame_C|SetRenderText (Variables|Default|GetGameMode) true)))
    (:then_1
      (if (< (.x (- _returnvalue _returnvalue_2)) 0.0)
        (if (<= (Math|Vector|Distance(Vector) _returnvalue _returnvalue_2) (Variables|/Game/BluePrint/InGame/BP_InGameChar.BP_InGameChar_C|GetSightRange (Variables|Default|GetTarget)))
          (Variables|/Game/BluePrint/InGame/BP_InGameChar.BP_InGameChar_C|SetOnBackMirror _target true))
        (else
          (Variables|/Game/BluePrint/InGame/BP_InGameChar.BP_InGameChar_C|SetOnBackMirror _target false))))))

(event Collision|EventHit
  (params (MyComp :type Primitive%20Component%20Object%20Reference) (Other :type Actor%20Object%20Reference) (OtherComp :type Primitive%20Component%20Object%20Reference) (bSelfMoved :type Boolean) (HitLocation :type Vector :default "0, 0, 0") (HitNormal :type Vector :default "0, 0, 0") (NormalImpulse :type Vector :default "0, 0, 0") (Hit :type Hit%20Result%20Structure%20%28by%20ref%29))
  (bind _gamemode (Variables|Default|GetGameMode))
  (bind _target (Variables|Default|GetTarget))
  (bind _gamemode_2 (Variables|Default|GetGameMode))
  (Audio|PlaySoundatLocation "/Game/Sound/Que_Explosion.Que_Explosion" HitLocation "0, 0, 0" 1.0 1.0 0.0 "/Game/Sound/At_Explosion.At_Explosion" 0 0 0)
  (Variables|Default|SetHit%20Location HitLocation)
  (if (Actor|ActorHasTag Other "Player")
    (if (Variables|/Game/BluePrint/InGame/BP_InGameChar.BP_InGameChar_C|GetCanHit (Variables|Default|GetTarget))
      (Variables|/Game/BluePrint/InGame/BP_InGameChar.BP_InGameChar_C|SetDamage _target (+ (Variables|/Game/BluePrint/InGame/BP_InGameChar.BP_InGameChar_C|GetDamage _target) 10))
      (Effects|SpawnEmitteratLocation "/Game/ExplosionA/Particles/Explosion/P_Explosion_Big_A.P_Explosion_Big_A" (+ (Variables|Default|GetHit%20Location) "1500.000000,0,0") "0, 0, 0" "3.000000,3.000000,3.000000")
      (Variables|/Game/BluePrint/InGame/BP_InGameChar.BP_InGameChar_C|SetGetForce (Variables|Default|GetTarget) true)
      (Variables|/Game/BluePrint/InGame/GM_InGame.GM_InGame_C|SetScore _gamemode_2 (- (Variables|/Game/BluePrint/InGame/GM_InGame.GM_InGame_C|GetScore _gamemode_2) 50))
      (else
        (Effects|SpawnEmitteratLocation "/Game/ExplosionSmke/Particles/Explosion/P_Explosion_Smoke.P_Explosion_Smoke" (+ (Variables|Default|GetHit%20Location) "1500.000000,0,0") "0, 0, 0" "3.000000,3.000000,3.000000")
        (Variables|/Game/BluePrint/InGame/GM_InGame.GM_InGame_C|SetScore _gamemode (+ (Variables|/Game/BluePrint/InGame/GM_InGame.GM_InGame_C|GetScore _gamemode) 50))))
    (Actor|DestroyActor)
    (Variables|/Game/BluePrint/InGame/BP_InGameChar.BP_InGameChar_C|SetOnBackMirror (Variables|Default|GetTarget) false)
    (Variables|/Game/BluePrint/InGame/GM_InGame.GM_InGame_C|SetRenderText (Variables|Default|GetGameMode) false)))

(fn ConstructionScript)