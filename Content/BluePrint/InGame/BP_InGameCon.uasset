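; Player controller for the in-game aircraft, driving BP_InGameChar's constant forward flight, steering and weapons.
; Axis input moves and tilts the plane while lerping wing and stabilizer angles in its AnimInstance; Turn plays a timeline roll with temporary invulnerability.
; LockOn gathers tagged enemies ahead within range, and Tick drops the lock once one falls behind.
; Missiles spawn per locked enemy with homing, or unguided otherwise, alongside timer-driven machine-gun fire.
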(event EventBeginPlay
  ;[1 1 1] Begin
  (bind _output_get (Variables|Default|SetFlyPlayer (Game|GetPlayerCharacter 0)))
  (bind _asbp_in_game_char (Utilities|Casting|CastToBP_InGameChar _output_get))
  (bind _output_get_2 (Variables|Default|SetChar _asbp_in_game_char))
  (Variables|Default|SetMovement (Variables|/Script/Engine.Character|GetCharacterMovement _output_get_2))
  (bind _asabp_in_game_char (Utilities|Casting|CastToABP_InGameChar (Components|SkeletalMesh|GetAnimInstance (Variables|/Script/Engine.Character|GetMesh (Variables|Default|GetChar)))))
  (Variables|Default|SetAnimInstance _asabp_in_game_char))

(event EventTick
  (params (DeltaSeconds :type Float%20%28single-precision%29))
  (Utilities|FlowControl|Sequence
    (:then_0
      (bind _output_get (Variables|Default|SetDelta%20Seconds DeltaSeconds))
      (Variables|Default|SetSecondPerFrame (+ (Variables|Default|GetSecondPerFrame) _output_get)))
    (:then_1
      (CallFunction|MoveFront))
    (:then_2
      (for _array_element (Variables|Default|GetEnemyInRange)
        (Utilities|IsValid _array_element
          (:Is%20Valid
            (if (not (> (.x (- (.location (Transformation|GetActorTransform _array_element)) (.location (Transformation|GetActorTransform (Variables|Default|GetChar))))) 0.0))
              (Variables|Default|SetIsTarget false)
              (Variables|Default|SetAiming false)
              (Variables|/Game/BluePrint/InGame/BP_Enemy.BP_Enemy_C|SetIsAiming (Variables|Default|GetTarget) false))))))))

(event Input|ActionEvents|InputActionTurn
  (params (Key :type Key%20Structure :default "None"))
  (bind _char (Variables|Default|GetChar))
  ;[1 1 1] Turn
  (:Pressed
    (if (not (Variables|/Game/BluePrint/InGame/BP_InGameChar.BP_InGameChar_C|GetIsBroken (Variables|Default|GetChar)))
      (if (not (Variables|Default|GetIsTurn))
        (bind _새_트랙_0 (Timeline|타임라인_0 PlayFromStart)
          (:Update
            (Variables|Default|SetIsTurn true)
            (Transformation|SetActorRotation _char (Math|Interpolation|RInterpTo (Pawn|GetControlRotation (Variables|Default|GetChar) :!class /Script/Engine.Pawn) "0, 0,180.000000" _새_트랙_0 0.5))
            (Variables|/Game/BluePrint/InGame/BP_InGameChar.BP_InGameChar_C|SetCanHit _char false))
          (:Finished
            (Timeline|타임라인_1 PlayFromStart
              (:Finished
                (Variables|Default|SetIsTurn false)
                (Utilities|FlowControl|Delay 1.0)
                (Variables|/Game/BluePrint/InGame/BP_InGameChar.BP_InGameChar_C|SetCanHit _char true)))))))))

(event Input|ActionEvents|InputActionGunFire
  (params (Key :type Key%20Structure :default "None"))
  (bind _char (Variables|Default|GetChar))
  (bind _machinegunfire (Variables|/Game/BluePrint/InGame/BP_InGameChar.BP_InGameChar_C|GetMachineGunFire _char))
  ;[1 1 1] GunFire
  (:Pressed
    (if (not (Variables|/Game/BluePrint/InGame/BP_InGameChar.BP_InGameChar_C|GetIsBroken (Variables|Default|GetChar)))
      (Variables|Default|SetGunFire true)
      (Components|Activation|Activate _machinegunfire true)
      (Utilities|Time|SetTimerbyFunctionName (Variables|Default|GetChar) "SetBullet" 0.2 true)))
  (:Released
    (Variables|Default|SetGunFire false)
    (Components|Activation|Deactivate _machinegunfire)))

(event Input|ActionEvents|InputActionMissilleFire
  (params (Key :type Key%20Structure :default "None"))
  ;[1 1 1] Projectille
  (:Pressed
    (if (not (Variables|/Game/BluePrint/InGame/BP_InGameChar.BP_InGameChar_C|GetIsBroken (Variables|Default|GetChar)))
      (if (not (Variables|Default|GetIsFire))
        (if (Variables|Default|GetIsTarget)
          (for _array_element (Variables|Default|GetEnemyInRange)
            (Utilities|IsValid _array_element
              (:Is%20Valid
                (bind _returnvalue (Game|SpawnActorfromClass "/Game/BluePrint/InGame/PlayerProj.PlayerProj_C" (Transformation|GetSocketTransform (Variables|/Script/Engine.Character|GetMesh (Variables|Default|GetChar)) (Variables|Default|GetIn%20Socket%20Name) "RTS_World") "AlwaysSpawn" 0 0))
                (bind _output_get (Variables|Default|SetPlayerProj _returnvalue))
                (Variables|/Script/Engine.ProjectileMovementComponent|SetHomingTargetComponent (Variables|/Game/BluePrint/InGame/PlayerProj.PlayerProj_C|GetProjectileMovement _output_get) (Variables|/Script/Engine.Actor|GetRootComponent _array_element))
                (Variables|/Script/Engine.ProjectileMovementComponent|SetbIsHomingProjectile (Variables|/Game/BluePrint/InGame/PlayerProj.PlayerProj_C|GetProjectileMovement _output_get) true)
                (Variables|/Script/Engine.ProjectileMovementComponent|SetHomingAccelerationMagnitude (Variables|/Game/BluePrint/InGame/PlayerProj.PlayerProj_C|GetProjectileMovement _output_get) 4e+04)
                (Transformation|SetActorRotation (Variables|Default|GetPlayerProj) (Math|Rotator|FindLookatRotation (Transformation|GetActorLocation (Variables|Default|GetPlayerProj)) (Transformation|GetActorLocation (Variables|Default|GetTarget))) true))))
          (Variables|Default|SetIsFire true)
          (else
            (Game|SpawnActorfromClass "/Game/BluePrint/InGame/PlayerProj.PlayerProj_C" (Transformation|GetSocketTransform (Variables|/Script/Engine.Character|GetMesh (Variables|Default|GetChar)) (Variables|Default|GetIn%20Socket%20Name) "RTS_World") "Undefined" 0 0)
            (Variables|Default|SetIsFire true))))))
  (:Released
    (Utilities|FlowControl|Delay 1.0)
    (Variables|Default|SetIsFire false)))

(event Input|ActionEvents|InputActionLockOn
  (params (Key :type Key%20Structure :default "None"))
  (bind _char (Variables|Default|GetChar))
  (bind _enemyinrange (Variables|Default|GetEnemyInRange))
  (bind _returnvalue (Transformation|GetActorTransform _char))
  ;[1 1 1] LockOn
  (:Pressed
    (if (not (Variables|/Game/BluePrint/InGame/BP_InGameChar.BP_InGameChar_C|GetIsBroken (Variables|Default|GetChar)))
      (bind _outactors (Actor|GetAllActorswithTag (Variables|Default|GetTagName)))
      (bind _output_get (Variables|Default|SetAllEnemyArray _outactors))
      (for _array_element _output_get
        (Variables|Default|SetEnemy%20Element _array_element)
        (if (> (.x (- (.location (Transformation|GetActorTransform _array_element)) (.location _returnvalue))) 0.0)
          (if (< (Math|Vector|Distance(Vector) (.location (Transformation|GetActorTransform _array_element)) (.location _returnvalue)) (Variables|/Game/BluePrint/InGame/BP_InGameChar.BP_InGameChar_C|GetRange (Variables|Default|GetChar)))
            (Audio|Components|Audio|Play (Variables|Default|GetLockOn) 0.0)
            (bind _asbp_enemy (Utilities|Casting|CastToBP_Enemy (Variables|Default|GetEnemy%20Element)))
            (bind _output_get_2 (Variables|Default|SetTarget _asbp_enemy))
            (Variables|/Game/BluePrint/InGame/BP_Enemy.BP_Enemy_C|SetIsAiming _output_get_2 true)
            (Utilities|Array|Add _enemyinrange (Variables|Default|GetEnemy%20Element))
            (if (!= (Utilities|Array|Length _enemyinrange) 0)
              (Variables|Default|SetIsTarget true)
              (Variables|Default|SetAiming true)
              (else
                (Variables|Default|SetIsTarget false)
                (Variables|Default|SetAiming false)
                (Variables|/Game/BluePrint/InGame/BP_Enemy.BP_Enemy_C|SetIsAiming (Variables|Default|GetTarget) false))))))))
  (:Released
    (Audio|Components|Audio|Stop (Variables|Default|GetLockOn))
    (for _array_element_2 (Variables|Default|GetEnemyInRange)
      (Utilities|IsValid _array_element_2
        (:Is%20Valid
          (bind _asbp_enemy_2 (Utilities|Casting|CastToBP_Enemy _array_element_2))
          (Variables|/Game/BluePrint/InGame/BP_Enemy.BP_Enemy_C|SetIsAiming _asbp_enemy_2 false))))
    (Utilities|Array|Clear (Variables|Default|GetAllEnemyArray))
    (Utilities|Array|Clear (Variables|Default|GetEnemyInRange))
    (Variables|Default|SetIsTarget false)
    (Variables|Default|SetAiming false)))

(event Input|AxisEvents|InputAxisUp/Down
  (params (AxisValue :type Float%20%28single-precision%29))
  (bind _char (Variables|Default|GetChar))
  ;[1 1 1] Up/Down
  (if (Variables|Default|GetInTrigger)
    (if (not (Variables|/Game/BluePrint/InGame/BP_InGameChar.BP_InGameChar_C|GetIsBroken (Variables|Default|GetChar)))
      (CallFunction|StabilizerAngle AxisValue)
      (CallFunction|RotationUpDown AxisValue)
      (Pawn|Input|AddMovementInput _char (Math|Vector|GetUpVector (Variables|/Script/Engine.Character|GetMesh _char)) AxisValue false))))

(event Input|AxisEvents|InputAxisRight/Left
  (params (AxisValue :type Float%20%28single-precision%29))
  (bind _char (Variables|Default|GetChar))
  (bind _returnvalue (Pawn|GetControlRotation _char :!class /Script/Engine.Pawn))
  ;[1 1 1] Right/Left
  (if (Variables|Default|GetInTrigger)
    (if (not (Variables|/Game/BluePrint/InGame/BP_InGameChar.BP_InGameChar_C|GetIsBroken (Variables|Default|GetChar)))
      (CallFunction|WingsAngle AxisValue)
      (CallFunction|RotationRightLeft AxisValue)
      (Pawn|Input|AddMovementInput _char (Math|Vector|GetRightVector (Math|Rotator|MakeRotator (.roll _returnvalue) 0.0 (.yaw _returnvalue))) AxisValue false))))

(fn ConstructionScript)

(fn StabilizerAngle
  (params (Axis :type Float%20%28double-precision%29))
  (bind _animinstance (Variables|Default|GetAnimInstance))
  (bind _animinstance_2 (Variables|Default|GetAnimInstance))
  (bind _animinstance_3 (Variables|Default|GetAnimInstance))
  (bind _delta_seconds (Variables|Default|GetDelta%20Seconds))
  (bind _animinstance_4 (Variables|Default|GetAnimInstance))
  (Variables|Default|SetLerpSpeed (* (Variables|Default|GetDelta%20Seconds) 1e+01))
  (switch int (Math|Float|Truncate Axis)
    (:-1
      (Variables|/Game/Animation/ABP_InGameChar.ABP_InGameChar_C|SetStabilizerLAngle (Variables|Default|GetAnimInstance) (Math|Float|Lerp (Variables|/Game/Animation/ABP_InGameChar.ABP_InGameChar_C|GetStabilizerLAngle _animinstance_4) 2e+01 (Variables|Default|GetLerpSpeed)))
      (Variables|/Game/Animation/ABP_InGameChar.ABP_InGameChar_C|SetStabilizerRAngle (Variables|Default|GetAnimInstance) (Math|Float|Lerp (Variables|/Game/Animation/ABP_InGameChar.ABP_InGameChar_C|GetStabilizerRAngle _animinstance_4) 2e+01 (Variables|Default|GetLerpSpeed))))
    (:0
      (Variables|/Game/Animation/ABP_InGameChar.ABP_InGameChar_C|SetStabilizerLAngle (Variables|Default|GetAnimInstance) (Math|Float|Lerp (Variables|/Game/Animation/ABP_InGameChar.ABP_InGameChar_C|GetStabilizerLAngle _animinstance_3) 0.0 _delta_seconds))
      (Variables|/Game/Animation/ABP_InGameChar.ABP_InGameChar_C|SetStabilizerRAngle (Variables|Default|GetAnimInstance) (Math|Float|Lerp (Variables|/Game/Animation/ABP_InGameChar.ABP_InGameChar_C|GetStabilizerRAngle _animinstance_3) 0.0 _delta_seconds)))
    (:1
      (Variables|/Game/Animation/ABP_InGameChar.ABP_InGameChar_C|SetStabilizerLAngle _animinstance_2 (Math|Float|Lerp (Variables|/Game/Animation/ABP_InGameChar.ABP_InGameChar_C|GetStabilizerLAngle _animinstance) -2e+01 (Variables|Default|GetLerpSpeed)))
      (Variables|/Game/Animation/ABP_InGameChar.ABP_InGameChar_C|SetStabilizerRAngle _animinstance_2 (Math|Float|Lerp (Variables|/Game/Animation/ABP_InGameChar.ABP_InGameChar_C|GetStabilizerRAngle _animinstance) -2e+01 (Variables|Default|GetLerpSpeed))))))

(fn RotationUpDown
  (params (Axis :type Float%20%28double-precision%29))
  (bind _char (Variables|Default|GetChar))
  (bind _char_2 (Variables|Default|GetChar))
  (bind _char_3 (Variables|Default|GetChar))
  (switch int (Math|Float|Truncate Axis)
    (:-1
      (Transformation|SetActorRotation _char_2 (Math|Interpolation|RInterpTo (Transformation|GetActorRotation _char_2) "-40.000000, 0, 0" (Variables|Default|GetDelta%20Seconds) 1.0)))
    (:0
      (Transformation|SetActorRotation _char_3 (Math|Interpolation|RInterpTo (Transformation|GetActorRotation _char_3) "0, 0, 0" (Variables|Default|GetDelta%20Seconds) 1.0)))
    (:1
      (Transformation|SetActorRotation _char (Math|Interpolation|RInterpTo (Transformation|GetActorRotation _char) "40.000000, 0, 0" (Variables|Default|GetDelta%20Seconds) 1.0)))))

(fn WingsAngle
  (params (Axis :type Float%20%28double-precision%29))
  (bind _animinstance (Variables|Default|GetAnimInstance))
  (bind _delta_seconds (Variables|Default|GetDelta%20Seconds))
  (switch int (Math|Float|Truncate Axis)
    (:-1
      (Variables|/Game/Animation/ABP_InGameChar.ABP_InGameChar_C|SetLWingsAngle _animinstance (Math|Float|Lerp (Variables|/Game/Animation/ABP_InGameChar.ABP_InGameChar_C|GetLWingsAngle _animinstance) -4e+01 (Variables|Default|GetDelta%20Seconds)))
      (Variables|/Game/Animation/ABP_InGameChar.ABP_InGameChar_C|SetRWingsAngle _animinstance (Math|Float|Lerp (Variables|/Game/Animation/ABP_InGameChar.ABP_InGameChar_C|GetRWingsAngle _animinstance) 4e+01 (Variables|Default|GetDelta%20Seconds))))
    (:0
      (Variables|/Game/Animation/ABP_InGameChar.ABP_InGameChar_C|SetLWingsAngle _animinstance (Math|Float|Lerp (Variables|/Game/Animation/ABP_InGameChar.ABP_InGameChar_C|GetLWingsAngle _animinstance) 0.0 (Variables|Default|GetDelta%20Seconds)))
      (Variables|/Game/Animation/ABP_InGameChar.ABP_InGameChar_C|SetRWingsAngle _animinstance (Math|Float|Lerp (Variables|/Game/Animation/ABP_InGameChar.ABP_InGameChar_C|GetRWingsAngle _animinstance) 0.0 (Variables|Default|GetDelta%20Seconds))))
    (:1
      (Variables|/Game/Animation/ABP_InGameChar.ABP_InGameChar_C|SetLWingsAngle _animinstance (Math|Float|Lerp (Variables|/Game/Animation/ABP_InGameChar.ABP_InGameChar_C|GetLWingsAngle _animinstance) 4e+01 _delta_seconds))
      (Variables|/Game/Animation/ABP_InGameChar.ABP_InGameChar_C|SetRWingsAngle _animinstance (Math|Float|Lerp (Variables|/Game/Animation/ABP_InGameChar.ABP_InGameChar_C|GetRWingsAngle _animinstance) -4e+01 _delta_seconds)))))

(fn RotationRightLeft
  (params (Axis :type Float%20%28double-precision%29))
  (bind _char (Variables|Default|GetChar))
  (bind _char_2 (Variables|Default|GetChar))
  (bind _char_3 (Variables|Default|GetChar))
  (switch int (Math|Float|Truncate Axis)
    (:-1
      (Transformation|SetActorRotation _char_2 (Math|Interpolation|RInterpTo (Transformation|GetActorRotation _char_2) "0.000000, 0,-60.000000" (Variables|Default|GetDelta%20Seconds) 1.0)))
    (:0
      (Transformation|SetActorRotation _char_3 (Math|Interpolation|RInterpTo (Transformation|GetActorRotation _char_3) "0, 0, 0" (Variables|Default|GetDelta%20Seconds) 1.0)))
    (:1
      (Transformation|SetActorRotation _char (Math|Interpolation|RInterpTo (Transformation|GetActorRotation _char) "0.000000, 0,60.000000" (Variables|Default|GetDelta%20Seconds) 1.0)))))

(fn MoveFront
  (bind _char (Variables|Default|GetChar))
  (Pawn|Input|AddMovementInput _char (Math|Vector|GetForwardVector (Math|Rotator|MakeRotator 0.0 0.0 (.yaw (Pawn|GetControlRotation _char :!class /Script/Engine.Pawn)))) 1.0 false))

(fn Test
  (Development|PrintString "Hello"))