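; Player rocket projectile that can home on a target, kills enemies on hit and expires after a fixed lifespan.
; BeginPlay caches game instance, player and game mode, creates a hit widget and starts the trail effect and rocket sound.
; Tick destroys it if its homing target becomes invalid.
; Any hit plays explosion audio and flags nearby players for force; enemy hits also remove the aim widget, spawn an explosion and update score.
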(event EventBeginPlay
  (Actor|SetLifeSpan 1e+01)
  (Components|Activation|SetActive (Variables|Default|GetNiagara) true false)
  (bind _asbp_game_inst (Utilities|Casting|CastToBP_GameInst (Game|GetGameInstance)))
  (Variables|Default|SetGameInst _asbp_game_inst)
  (bind _asbp_in_game_char (Utilities|Casting|CastToBP_InGameChar (Game|GetPlayerCharacter 0)))
  (Variables|Default|SetPlayer _asbp_in_game_char)
  (bind _asgm_in_game (Utilities|Casting|CastToGM_InGame (Game|GetGameMode)))
  (Variables|Default|SetGM _asgm_in_game)
  (bind _returnvalue (UserInterface|CreateWidget "/Game/UI/BP_HitUi.BP_HitUi_C"))
  (Variables|Default|SetNewVar_0 _returnvalue)
  (Audio|Components|Audio|Play (Variables|Default|GetRocketSound) 0.0))

(event Collision|EventActorBeginOverlap
  (params (OtherActor :type Actor%20Object%20Reference)))

(event EventTick
  (params (DeltaSeconds :type Float%20%28single-precision%29))
  (bind _projectilemovement (Variables|Default|GetProjectileMovement))
  (if (Variables|/Script/Engine.ProjectileMovementComponent|GetbIsHomingProjectile _projectilemovement)
    (Utilities|IsValid (Variables|/Script/Engine.ProjectileMovementComponent|GetHomingTargetComponent _projectilemovement)
      (:Is%20Not%20Valid
        (Actor|DestroyActor)))))

(event Collision|EventHit
  (params (MyComp :type Primitive%20Component%20Object%20Reference) (Other :type Actor%20Object%20Reference) (OtherComp :type Primitive%20Component%20Object%20Reference) (bSelfMoved :type Boolean) (HitLocation :type Vector :default "0, 0, 0") (HitNormal :type Vector :default "0, 0, 0") (NormalImpulse :type Vector :default "0, 0, 0") (Hit :type Hit%20Result%20Structure%20%28by%20ref%29))
  (bind _gm (Variables|Default|GetGM))
  (Audio|PlaySoundatLocation "/Game/Sound/Que_Explosion.Que_Explosion" (Transformation|GetActorLocation) "0, 0, 0" 1.0 1.0 0.0 "/Game/Sound/At_Explosion.At_Explosion" 0 0 0)
  (if (<= (Math|Vector|Distance(Vector) HitLocation (Transformation|GetActorLocation (Variables|Default|GetPlayer))) 5e+04)
    (Variables|/Game/BluePrint/InGame/BP_InGameChar.BP_InGameChar_C|SetGetForce (Variables|Default|GetPlayer) true))
  (Actor|DestroyActor)
  (if (Actor|ActorHasTag Other "Enemy")
    (bind _asbp_enemy (Utilities|Casting|CastToBP_Enemy Other))
    (Widget|RemovefromParent (Variables|/Game/BluePrint/InGame/BP_Enemy.BP_Enemy_C|GetAim _asbp_enemy))
    (Actor|DestroyActor Other)
    (bind _returnvalue (Effects|SpawnEmitteratLocation "/Game/ExplosionB/Particles/Explosion/P_Explosion_Big_B.P_Explosion_Big_B" HitLocation "0, 0, 0" "15.000000,15.000000,15.000000"))
    (Effects|Components|ParticleSystem|SetVectorParameter _returnvalue "Target" "0, 0, 0")
    (Variables|/Game/BluePrint/InGame/GM_InGame.GM_InGame_C|SetScore _gm (+ (Variables|/Game/BluePrint/InGame/GM_InGame.GM_InGame_C|GetScore _gm) 100))
    (Variables|/Game/BluePrint/InGame/GM_InGame.GM_InGame_C|SetIsProjHit _gm true)))

(fn ConstructionScript)