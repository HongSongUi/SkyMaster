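; Player F-18C fighter jet character that flies in Flying movement mode, with thruster effects, flight sound and a glowing dynamic material.
; BeginPlay caches the anim instance and controller; WingsAngle lerps wing angles on the anim instance.
; Tick manages timed force/camera-shake and miss flags, and at 100 damage marks the jet broken and spawns wreckage.
; SetBullet spawns bullets at the controller's chosen socket; PlayToggle pauses the game.
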(event EventBeginPlay
  (Pawn|Components|CharacterMovement|SetMovementMode (Variables|Character|GetCharacterMovement) "MOVE_Flying" 0)
  (Rendering|Material|SetScalarParameterValue (Variables|Default|GetLight) "Emission" 1e+02 :!class /Script/Engine.MaterialInstanceDynamic)
  (CallFunction|SetEffect)
  (bind _asabp_in_game_char (Utilities|Casting|CastToABP_InGameChar (Components|SkeletalMesh|GetAnimInstance (Variables|Character|GetMesh))))
  (Variables|Default|SetAnimInstance _asabp_in_game_char)
  (bind _asbp_in_game_con (Utilities|Casting|CastToBP_InGameCon (Pawn|GetController)))
  (Variables|Default|SetControl _asbp_in_game_con)
  (Variables|Default|SetRange 1e+05)
  (Variables|Default|SetCanHit true)
  (Components|SkinnedMesh|SetPhysicsAsset (Variables|Character|GetMesh) "/Game/InGameVigilante/Vehicles/West_Fighter_F18C/PHYS_West_Fighter_F18C.PHYS_West_Fighter_F18C" false)
  (Rendering|SetVisibility (Variables|Default|GetDamaged) false false)
  (Audio|PlaySoundatLocation "/Game/Sound/Que_FlightSound.Que_FlightSound" (Transformation|GetActorLocation) "0, 0, 0" 1.0 1.0 0.0 0 0 0 0))

(event Collision|EventActorBeginOverlap
  (params (OtherActor :type Actor%20Object%20Reference)))

(event EventTick
  (params (DeltaSeconds :type Float%20%28single-precision%29))
  (Utilities|FlowControl|Sequence
    (:then_0
      (Variables|Default|SetDelta%20Seconds DeltaSeconds))
    (:then_1
      (if (Variables|Default|GetGetForce)
        (Variables|Default|SetCamShake 0)
        (Utilities|FlowControl|Delay 1.0)
        (Variables|Default|SetGetForce false)
        (else
          (Variables|Default|SetCamShake 1))))
    (:then_2
      (if (>= (Variables|Default|GetDamage) 100)
        (Variables|Default|SetIsBroken true)
        (Effects|SpawnEmitteratLocation "/Game/FireParticle/Vehicles/West_Fighter_F18C/FX/FX_Wreckage_01_F18C.FX_Wreckage_01_F18C" (Transformation|GetActorLocation))))
    (:then_3
      (if (Variables|Default|GetIsMiss)
        (Utilities|FlowControl|Delay 1.0)
        (Variables|Default|SetIsMiss false)))))

(event Collision|EventHit
  (params (MyComp :type Primitive%20Component%20Object%20Reference) (Other :type Actor%20Object%20Reference) (OtherComp :type Primitive%20Component%20Object%20Reference) (bSelfMoved :type Boolean) (HitLocation :type Vector :default "0, 0, 0") (HitNormal :type Vector :default "0, 0, 0") (NormalImpulse :type Vector :default "0, 0, 0") (Hit :type Hit%20Result%20Structure%20%28by%20ref%29)))

(event Input|ActionEvents|InputActionPlayToggle
  (params (Key :type Key%20Structure :default "None"))
  (:Pressed
    (bind _output_get (Variables|Default|SetGamePause (not (Variables|Default|GetGamePause))))
    (Game|SetGamePaused _output_get)))

(fn ConstructionScript
  (|CallParentFunction)
  (bind _returnvalue (Rendering|Material|CreateDynamicMaterialInstance (Variables|Character|GetMesh) 0 0 "None" :!class /Script/Engine.PrimitiveComponent))
  (Variables|Default|SetLight _returnvalue))

(fn SetEffect
  (bind _mesh (Variables|Character|GetMesh))
  (Utilities|IsValid (Variables|컴포넌트|GetLeftFire)
    (:Is%20Not%20Valid
      (Utilities|IsValid (Variables|컴포넌트|GetRightFire)
        (:Is%20Not%20Valid
          (Utilities|FlowControl|Sequence
            (:then_0
              (bind _returnvalue (Effects|SpawnEmitterAttached "/Game/InGameVigilante/Vehicles/West_Fighter_F18C/FX/FX_Engine_01_F18C.FX_Engine_01_F18C" _mesh "lf_thruster_jntSocket"))
              (Variables|컴포넌트|SetLeftFire _returnvalue))
            (:then_1
              (bind _returnvalue_2 (Effects|SpawnEmitterAttached "/Game/InGameVigilante/Vehicles/West_Fighter_F18C/FX/FX_Engine_01_F18C.FX_Engine_01_F18C" _mesh "rt_thruster_jntSocket"))
              (Variables|컴포넌트|SetRightFire _returnvalue_2))))))))

(fn WingsAngle
  (params (A :type Float%20%28double-precision%29))
  (bind _animinstance (Variables|Default|GetAnimInstance))
  (bind _animinstance_2 (Variables|Default|GetAnimInstance))
  (bind _animinstance_3 (Variables|Default|GetAnimInstance))
  (bind _delta_seconds (Variables|Default|GetDelta%20Seconds))
  (bind _animinstance_4 (Variables|Default|GetAnimInstance))
  ;[1 1 1] UP/Down Wings
  (switch int (Math|Float|Truncate A)
    (:-1
      (Variables|/Game/Animation/ABP_InGameChar.ABP_InGameChar_C|SetLWingsAngle (Variables|Default|GetAnimInstance) (Math|Float|Lerp (Variables|/Game/Animation/ABP_InGameChar.ABP_InGameChar_C|GetLWingsAngle _animinstance_4) -4e+01 (Variables|Default|GetDelta%20Seconds)))
      (Variables|/Game/Animation/ABP_InGameChar.ABP_InGameChar_C|SetRWingsAngle (Variables|Default|GetAnimInstance) (Math|Float|Lerp (Variables|/Game/Animation/ABP_InGameChar.ABP_InGameChar_C|GetRWingsAngle _animinstance_4) -4e+01 (Variables|Default|GetDelta%20Seconds))))
    (:0
      (Variables|/Game/Animation/ABP_InGameChar.ABP_InGameChar_C|SetLWingsAngle (Variables|Default|GetAnimInstance) (Math|Float|Lerp (Variables|/Game/Animation/ABP_InGameChar.ABP_InGameChar_C|GetLWingsAngle _animinstance_3) 0.0 (Variables|Default|GetDelta%20Seconds)))
      (Variables|/Game/Animation/ABP_InGameChar.ABP_InGameChar_C|SetRWingsAngle (Variables|Default|GetAnimInstance) (Math|Float|Lerp (Variables|/Game/Animation/ABP_InGameChar.ABP_InGameChar_C|GetRWingsAngle _animinstance_3) 0.0 (Variables|Default|GetDelta%20Seconds))))
    (:1
      (Variables|/Game/Animation/ABP_InGameChar.ABP_InGameChar_C|SetLWingsAngle _animinstance_2 (Math|Float|Lerp (Variables|/Game/Animation/ABP_InGameChar.ABP_InGameChar_C|GetLWingsAngle _animinstance) 4e+01 _delta_seconds))
      (Variables|/Game/Animation/ABP_InGameChar.ABP_InGameChar_C|SetRWingsAngle _animinstance_2 (Math|Float|Lerp (Variables|/Game/Animation/ABP_InGameChar.ABP_InGameChar_C|GetRWingsAngle _animinstance) 4e+01 _delta_seconds)))))

(fn Test
  (Development|PrintString "Hello"))

(fn SetBullet
  (if (Variables|/Game/BluePrint/InGame/BP_InGameCon.BP_InGameCon_C|GetGunFire (Variables|Default|GetControl))
    (Game|SpawnActorfromClass "/Game/BluePrint/InGame/BP_Bullet.BP_Bullet_C" (Transformation|GetSocketTransform (Variables|Character|GetMesh) (Variables|/Game/BluePrint/InGame/BP_InGameCon.BP_InGameCon_C|GetAttach%20Point%20Name (Variables|Default|GetControl)) "RTS_World") "Undefined" self 0)))