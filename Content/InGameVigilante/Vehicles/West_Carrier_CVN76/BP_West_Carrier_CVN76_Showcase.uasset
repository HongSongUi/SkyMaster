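; Showcase Blueprint of the West Carrier CVN76 aircraft carrier that exposes the ship's animated parts to slider and checkbox controls.
; BeginPlay starts the radars spinning and zeroes two rear turret rotations.
; Slider events forward values to parent setters for lights, rudder, propellers, lifts, deflectors, and grouped turret and searchlight elevation and rotation.
; A checkbox toggles the damaged look.
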(event EventBeginPlay
  (|CallParentFunction)
  (CallFunction|SetMainRadarSpeed 1.0)
  (CallFunction|SetRadarSpeed 1.0)
  (CallFunction|SetLeftRearTurret2BaseRotation 0.0)
  (CallFunction|SetRightRearTurretBaseRotation 0.0))

(event Collision|EventActorBeginOverlap
  (params (OtherActor :type Actor%20Object%20Reference))
  (|CallParentFunction OtherActor) ; This node is disabled and will not be called.\nDrag off pins to build functionality.
)

(event EventSetTwinSliderVariable6
  (params (bFirstSlider? :type Boolean) (NewFirstValue :type Float%20%28double-precision%29) (NewSecondValue :type Float%20%28double-precision%29))
  (Utilities|FlowControl|Sequence
    (:then_0
      (CallFunction|SetLeftRearLightsElevation NewFirstValue)
      (CallFunction|SetRightRearLightsElevation NewFirstValue))
    (:then_1
      (CallFunction|SetLeftRearLightsBaseRotation NewSecondValue)
      (CallFunction|SetRightRearLightsBaseRotation NewSecondValue))))

(event EventSetCheckboxVariable0
  (params (NewState :type Boolean))
  (CallFunction|SetShowDamaged NewState))

(event EventSetSliderVariable1
  (params (NewValue :type Float%20%28double-precision%29))
  (CallFunction|SetRudder NewValue))

(event EventTick
  (params (DeltaSeconds :type Float%20%28single-precision%29))
  (|CallParentFunction DeltaSeconds) ; This node is disabled and will not be called.\nDrag off pins to build functionality.
)

(event EventSetTwinSliderVariable0
  (params (bFirstSlider? :type Boolean) (NewFirstValue :type Float%20%28double-precision%29) (NewSecondValue :type Float%20%28double-precision%29))
  (CallFunction|SetLeft1PropellerSpeed NewFirstValue)
  (CallFunction|SetLeft2PropellerSpeed NewFirstValue)
  (CallFunction|SetRight1PropellerSpeed NewSecondValue)
  (CallFunction|SetRight2PropellerSpeed NewSecondValue))

(event EventSetTwinSliderVariable1
  (params (bFirstSlider? :type Boolean) (NewFirstValue :type Float%20%28double-precision%29) (NewSecondValue :type Float%20%28double-precision%29))
  (CallFunction|SetLeftLift NewFirstValue)
  (CallFunction|SetRighttLift1 NewSecondValue))

(event EventSetSliderVariable0
  (params (NewValue :type Float%20%28double-precision%29))
  (CallFunction|SetLightsEmissivity NewValue))

(event EventSetTwinSliderVariable2
  (params (bFirstSlider? :type Boolean) (NewFirstValue :type Float%20%28double-precision%29) (NewSecondValue :type Float%20%28double-precision%29))
  (CallFunction|SetRighttLift2 NewFirstValue)
  (CallFunction|SetRighttLift3 NewSecondValue))

(event EventSetTwinSliderVariable3
  (params (bFirstSlider? :type Boolean) (NewFirstValue :type Float%20%28double-precision%29) (NewSecondValue :type Float%20%28double-precision%29))
  (CallFunction|SetDeflector1 NewFirstValue)
  (CallFunction|SetDeflector2 NewSecondValue))

(event EventSetTwinSliderVariable4
  (params (bFirstSlider? :type Boolean) (NewFirstValue :type Float%20%28double-precision%29) (NewSecondValue :type Float%20%28double-precision%29))
  (CallFunction|SetDeflector3 NewFirstValue)
  (CallFunction|SetDeflector4 NewSecondValue))

(event EventSetTwinSliderVariable5
  (params (bFirstSlider? :type Boolean) (NewFirstValue :type Float%20%28double-precision%29) (NewSecondValue :type Float%20%28double-precision%29))
  (Utilities|FlowControl|Sequence
    (:then_0
      (CallFunction|SetLeftFrontTurretElevation NewFirstValue)
      (CallFunction|SetLeftMidTurretElevation NewFirstValue)
      (CallFunction|SetLeftRearTurret1Elevation NewFirstValue)
      (CallFunction|SetLeftRearTurret2Elevation NewFirstValue)
      (CallFunction|SetRightFrontTurretElevation NewFirstValue)
      (CallFunction|SetRightRearTurretElevation NewFirstValue))
    (:then_1
      (CallFunction|SetLeftFrontTurretBaseRotation NewSecondValue)
      (CallFunction|SetLeftMidTurretBaseRotation NewSecondValue)
      (CallFunction|SetLeftRearTurret1BaseRotation NewSecondValue)
      (CallFunction|SetLeftRearTurret2BaseRotation NewSecondValue)
      (CallFunction|SetRightFrontTurretBaseRotation NewSecondValue)
      (CallFunction|SetRightRearTurretBaseRotation NewSecondValue))))

(fn ConstructionScript
  (|CallParentFunction))